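; Player controller for RTS-style ship selection and orders in space, with a free-look pawn camera.
; Axis inputs move the camera and adjust its speed, while mouse look works only with the cursor hidden.
; Click traces and HUD_FreeLook drag rectangles fill SelectedObjects, highlighted through custom depth.
; A short right-click toggles the HUD_Gameplay ship menu and stores the traced point that MoveSelectedActorsToPosition passes to selected ships.
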(event `self.ReceiveBeginPlay`
  ;[1 1 1] Enable HUD and set it as BP variable
  (bind _returnvalue (`|CreateWidget` "/Game/Space/HUD/HUD_Gameplay.HUD_Gameplay_C"))
  (bind _output_get (set `self.MainHUDRef` _returnvalue))
  (`UserWidget.AddToViewport` _output_get 0))

(event `Key|RightMouseButton`
  (params (Key :type "Key Structure"))
  (bind (_firstposition _secondposition) (break `/Game/Space/Utils/Structures/DoubleVector2D` (`self.CursorPositionChange`)))
  (bind (_locationx _locationy) (`self.GetMousePosition` (`GameplayStatics.GetPlayerController` 0)))
  (bind _returnvalue (`KismetMathLibrary.MakeVector2D` _locationx _locationy))
  ;[1 1 1] Control context menu/camera movement with Right Mouse Button
  (:`Pressed`
    (set `self.CursorPositionChange` (make `/Game/Space/Utils/Structures/DoubleVector2D` _returnvalue)))
  (:`Released`
    (set `self.CursorPositionChange` (make `/Game/Space/Utils/Structures/DoubleVector2D` _firstposition _returnvalue))
    (if (< (`KismetMathLibrary.Distance2D` _firstposition _secondposition) (`self.CursorRightClickThreshold`))
      (set `self.bShowMouseCursor` true)
      (`WidgetBlueprintLibrary.SetInputMode_GameAndUIEx` (`GameplayStatics.GetPlayerController` 0) null "DoNotLock" false)
      (if (> (`KismetArrayLibrary.Array_Length` (`self.SelectedObjects`)) 0)
        (`/Game/Space/HUD/HUD_Gameplay.ToggleShipContextMenu` (`self.MainHUDRef`))
        (bind (_startlocation _hitlocation) (`self.Trace for Object Under Cursor` 1000000.0))
        (set `self.LocationToMove` _hitlocation)))))

(event `MoveSelectedActorsToPosition`
  (for _array_element (`self.SelectedObjects`)
    (bind _asbp_ship (cast `/Game/Space/GameObjects/Ship/BP_Ship` _array_element))
    (`/Game/Space/GameObjects/Ship/BP_Ship.EventLookToPosition` _asbp_ship (`self.LocationToMove`))))

(event `InputAxis|CameraSpeed`
  (params (AxisValue :type "Float (single-precision)"))
  ;[1 1 1] Control camera movement speed (forward, backward and sideways only)
  (if (!= AxisValue 0.0)
    (bind _asbp_free_look (cast `/Game/Space/GameObjects/BP_FreeLook` (`GameplayStatics.GetPlayerPawn` 0)))
    (bind _floatingpawnmovement (`/Game/Space/GameObjects/BP_FreeLook.FloatingPawnMovement` _asbp_free_look))
    (bind _returnvalue (`KismetMathLibrary.FClamp` (+ (`MovementComponent.GetMaxSpeed` _floatingpawnmovement) (* AxisValue (`self.MoveIncrement`))) 250.0 100000.0))
    (set `FloatingPawnMovement.MaxSpeed` _returnvalue _floatingpawnmovement)
    (set `FloatingPawnMovement.Deceleration` (+ (* _returnvalue 5.0) 500.0) _floatingpawnmovement)))

(event `InputAxis|CameraMoveSideways`
  (params (AxisValue :type "Float (single-precision)"))
  ;[1 1 1] Move camera sideways
  (`Pawn.AddMovementInput` (`GameplayStatics.GetPlayerPawn` 0) (`KismetMathLibrary.GetRightVector` (`KismetMathLibrary.MakeRotator` 0.0 0.0 (.yaw (`self.GetControlRotation`)))) AxisValue false))

(event `InputAxis|CameraMoveForward`
  (params (AxisValue :type "Float (single-precision)"))
  ;[1 1 1] Move camera forward and backward
  (`Pawn.AddMovementInput` (`GameplayStatics.GetPlayerPawn` 0) (`KismetMathLibrary.GetForwardVector` (`KismetMathLibrary.MakeRotator` 0.0 (.pitch (`self.GetControlRotation`)) (.yaw (`self.GetControlRotation`)))) AxisValue false))

(event `InputAxis|CameraMoveUp`
  (params (AxisValue :type "Float (single-precision)"))
  ;[1 1 1] Move camera up and down
  (`Pawn.AddMovementInput` (`GameplayStatics.GetPlayerPawn` 0) (`KismetMathLibrary.GetUpVector` (`KismetMathLibrary.MakeRotator` 0.0 0.0 (.yaw (`self.GetControlRotation`)))) AxisValue false))

(event `Key|LeftMouseButton`
  (params (Key :type "Key Structure"))
  ;[1 1 1] Control mouse cursor visibility
  (:`Released`
    (`WidgetBlueprintLibrary.SetInputMode_GameOnly` (`GameplayStatics.GetPlayerController` 0) :!label _label)))

(event `InputAction|EnableMouseLook`
  (params (Key :type "Key Structure"))
  ;[1 1 1] Control mouse cursor visibility
  (:`Pressed`
    (set `self.bShowMouseCursor` false)
    (goto _label))
  (:`Released`
    (set `self.bShowMouseCursor` true)))

(event `InputAxis|CameraRotateZ (Yaw)`
  (params (AxisValue :type "Float (single-precision)"))
  ;[1 1 1] Control mouse cursor visibility
  (if (not (`self.bShowMouseCursor`))
    (`Pawn.AddControllerYawInput` (`GameplayStatics.GetPlayerPawn` 0) AxisValue)))

(event `InputAxis|CameraRotateY (Pitch)`
  (params (AxisValue :type "Float (single-precision)"))
  ;[1 1 1] Control mouse cursor visibility
  (if (not (`self.bShowMouseCursor`))
    (`Pawn.AddControllerPitchInput` (`GameplayStatics.GetPlayerPawn` 0) AxisValue)))

(event `InputAction|AddSelection`
  (params (Key :type "Key Structure"))
  (:`Pressed`
    (bind (_startlocation _hitlocation _outhitactor) (`self.Trace for Object Under Cursor` 1000000.0))
    (bind _out_actor (`self.IsValidSelection` _outhitactor)
      (:`Valid`
        (`self.SelectObject` _out_actor true)))))

(event `InputAction|SelectObject`
  (params (Key :type "Key Structure"))
  (:`Pressed`
    (bind (_startlocation _hitlocation _outhitactor) (`self.Trace for Object Under Cursor` 1000000.0))
    (bind _out_actor (`self.IsValidSelection` _outhitactor)
      (:`Valid`
        (`self.DeselectAllObjects`)
        (`self.SelectObject` _out_actor))
      (:`Invalid`
        (`self.DeselectAllObjects` :!label _label))
      (:`NotSelectable`
        (goto _label)))))

(event `Key|LeftMouseButton`
  (params (Key :type "Key Structure"))
  (bind _mainhudref (`self.MainHUDRef`))
  (bind (_locationx _locationy) (`self.GetMousePosition` self))
  (:`Pressed`
    (bind _ashud_free_look (cast `/Game/Space/HUD/HUD_FreeLook` (`self.GetHUD` self)))
    (`/Game/Space/HUD/HUD_FreeLook.Draw Rectangle` _ashud_free_look true (`KismetMathLibrary.MakeVector2D` _locationx _locationy) 2.0))
  (:`Released`
    (`/Game/Space/HUD/HUD_FreeLook.Draw Rectangle` _ashud_free_look false (0.0 0.0) 0.0)
    (`/Game/Space/HUD/HUD_Gameplay.SetWidgetVisibility` _mainhudref (`/Game/Space/HUD/HUD_Gameplay.HUD_ShipContextMenu` _mainhudref) "NewEnumerator3")))

(event `OnSelectionDrag`
  (params (FirstPoint :type "Vector2D Structure") (SecondPoint :type "Vector2D Structure"))
  (`self.SelectObjectsInRectangle` FirstPoint SecondPoint))

(fn `CheckForCursorSelection`
  (returns (OutHitActor :type "Actor Object Reference"))
  (bind (_startlocation _hitlocation _outhitactor) (`self.Trace for Object Under Cursor` 0.0))
  (return _outhitactor))

(fn `DeselectAllObjects`
  (for _array_element (`self.SelectedObjects`)
    (`self.SetHighlight` false _array_element))
  (set `self.SelectedObjects` (`|MakeArray`)))

(fn `DeselectObject`
  (params (Actor :type "Actor Object Reference"))
  (`self.IsValidSelection` Actor
    (:`Valid`
      (`KismetArrayLibrary.Array_RemoveItem` (`self.SelectedObjects`) Actor)
      (`self.SetHighlight` false Actor))))

(fn `SelectObject`
  (params (Actor :type "Actor Object Reference") (Toggle :type Boolean))
  (`self.IsValidSelection` Actor
    (:`Valid`
      (if (and Toggle (`KismetArrayLibrary.Array_Contains` (`self.SelectedObjects`) Actor))
        (`self.DeselectObject` Actor) ; Deselect item if it is includes in the list and toggle is ON
        (else
          (`self.SetHighlight` true Actor)
          (`KismetArrayLibrary.Array_Add` (`self.SelectedObjects`) Actor))))))

(fn `SelectObjectsInRectangle`
  (params (FirstPoint :type "Vector2D Structure (by ref)") (SecondPoint :type "Vector2D Structure (by ref)"))
  (`self.DeselectAllObjects`)
  (for _array_element (`HUD.GetActorsInSelectionRectangle` (`self.GetHUD` self) "/Game/Space/GameObjects/Ship/BP_Ship.BP_Ship_C" FirstPoint SecondPoint false true)
    (`self.SelectObject` _array_element)))

(fn `SetHighlight`
  (params (`HIghlight On` :type Boolean) (Actor :type "Actor Object Reference"))
  (`PrimitiveComponent.SetRenderCustomDepth` (`self.GetComponentByClass` Actor "/Script/Engine.MeshComponent") `HIghlight On`))

(fn `Trace for Object Under Cursor`
  (params (TraceDistance :type "Float (double-precision)" :default 1000000.0))
  (returns (StartLocation :type "Vector Structure") (HitLocation :type "Vector Structure") (OutHitActor :type "Actor Object Reference") (OutHit :type "HitResult Structure"))
  (bind (_worldlocation _worlddirection) (`self.DeprojectMousePositionToWorld` (`PlayerState.GetPlayerController` (`GameplayStatics.GetPlayerState` 0))))
  (bind _outhit (`KismetSystemLibrary.LineTraceSingle` _worldlocation (+ _worldlocation (* _worlddirection TraceDistance)) "TraceTypeQuery1"))
  (bind (_bblockinghit _binitialoverlap _time _distance _location _impactpoint _normal _impactnormal _physmat _hitactor) (`GameplayStatics.BreakHitResult` _outhit))
  (return _worldlocation _impactpoint _hitactor _outhit))

(fn `UserConstructionScript`)
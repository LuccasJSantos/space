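; Rocket actor that flies along its arrow's forward axis toward a target and tries to stop on it, then turns the target's material green.
; Tick runs an Accelerate, Brake, Wait state machine whose throttle becomes a clamped physics force on the cone.
; A PID on signed distance drives acceleration up to a speed limit.
; Braking starts near the kinematic stopping distance and scales with remaining distance against it; Wait zeroes velocity.
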(event `self.ReceiveBeginPlay`)

(event `self.ReceiveTick`
  (params (DeltaSeconds :type "Float (single-precision)"))
  (switch `/Game/PID/EShipState` (`self.State`)
    (:`NewEnumerator0`
      (`self.Check For Brake`)
      (`self.AccelControl (PID)` DeltaSeconds)
      (`self.ThrottleToForce` DeltaSeconds :!label _label))
    (:`NewEnumerator1`
      (`self.BrakeControl` DeltaSeconds)
      (goto _label))
    (:`NewEnumerator2`
      (`self.WaitControl`)
      (`|ExecutionSequence`
        (:`then_0`
          (goto _label))
        (:`then_1`
          (`PrimitiveComponent.SetMaterial` (`self.GetComponentByClass` (`self.Target`) "/Script/Engine.StaticMeshComponent") 0 "/Game/PID/ClothMaterialGreen.ClothMaterialGreen"))))))

(fn `AccelControl (PID)`
  (params (DeltaSeconds :type "Float (double-precision)"))
  (bind _output (`/Game/Space/Utils/Classes/PID.Get Output (Float)` (`self.PIDThrottle`) (* (`self.GetDistanceToTarget`) (`KismetMathLibrary.Dot_VectorVector` (`KismetMathLibrary.Normal` (- (`self.K2_GetActorLocation` (`self.Target`)) (`self.K2_GetActorLocation`))) (`KismetMathLibrary.Normal` (`SceneComponent.GetForwardVector` (`self.Arrow`))))) DeltaSeconds))
  (set `self.Throttle` _output))

(fn `BrakeControl`
  (params (DeltaSeconds :type "Float (double-precision)"))
  (bind _distance (`self.GetDistanceToTarget`))
  (if (`KismetMathLibrary.NearlyEqual_FloatFloat` _distance 0.0 0.01)
    (set `self.State` "NewEnumerator2")
    (else
      (bind _result (`|MagicNode` (`self.Speed`) (/ (`KismetMathLibrary.VSize` (`self.GetVelocity` (`self.Target`))) 100.0) (`self.Deceleration`)))
      (set `self.Throttle` (`KismetMathLibrary.FClamp` (* -1.0 (+ (- 1.0 (/ _distance _result)) 1.0)) -1.1 1.0)))))

(fn `Check For Brake`
  (`/Engine/EditorBlueprintResources/StandardMacros.IsValid` (`self.Target`)
    (:`Is Valid`
      (bind _result (`|MagicNode` (`self.Speed`) 0.0 (`self.Deceleration`)))
      (if (`KismetMathLibrary.NearlyEqual_FloatFloat` _result (`self.GetDistanceToTarget`) (`KismetMathLibrary.FMax` (`self.Deceleration`) (`self.Acceleration`)))
        (set `self.State` "NewEnumerator1")))))

(fn `Get Speed`
  (returns (Speed :type "Float (double-precision)"))
  (return (/ (`KismetMathLibrary.VSize` (`self.GetVelocity`)) 100.0)))

(fn `GetDistanceToTarget`
  (returns (Distance :type "Float (double-precision)"))
  (return (/ (`KismetMathLibrary.Vector_Distance` (`self.K2_GetActorLocation` (`self.Target`)) (`self.K2_GetActorLocation`)) 100.0)))

(fn `ThrottleToForce`
  (params (DeltaSeconds :type "Float (double-precision)"))
  (`PrimitiveComponent.AddForce` (`self.Cone`) (* 100.0 (`/Game/Space/Utils/SpaceGame.Clamp Range Band` (* (select `/Game/PID/EShipState` (`self.State`) :`NewEnumerator0` (select `bool` (>= (`self.Speed`) (`self.MaxSpeed`)) :`false` (`self.Acceleration`)) :`NewEnumerator1` (`self.Deceleration`)) (`self.Throttle`)) -0.3 0.3) (`SceneComponent.GetForwardVector` (`self.Arrow`))) "None" true)
  (set `self.Speed` (`self.Get Speed`)))

(fn `UserConstructionScript`)

(fn `WaitControl`
  (set `self.Throttle` 0.0)
  (`PrimitiveComponent.SetPhysicsLinearVelocity` (`self.Cone`) (0.0 0.0 0.0) false "None"))